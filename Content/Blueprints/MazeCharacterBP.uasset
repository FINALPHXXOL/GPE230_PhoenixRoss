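; MazeCharacterBP is the maze player character, with a stun ability against NPC enemies.
; On BeginPlay it adds the HUD widget to the viewport and hides the cursor.
; Stun input, gated by a cooldown counted down in Tick, fires particles and sphere-traces around the character, calling Stunned on NPCEnemyBP hits.
; GetStunCooldown returns a constant zero, and the P key only casts the game mode.
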(event EventBeginPlay
  (bind _returnvalue (UserInterface|CreateWidget "/Game/Blueprints/UI/HUDWidget.HUDWidget_C"))
  (bind _output_get (Variables|Default|SetHUD%20UI _returnvalue))
  (UserInterface|Viewport|AddtoViewport _output_get 0)
  (Variables|/Script/Engine.PlayerController|SetbShowMouseCursor (Game|GetPlayerController 0) false))

(event EventTick
  (params (DeltaSeconds :type Float%20%28single-precision%29))
  (if (> (Variables|Default|GetStunCooldown) 0.0)
    (Variables|Default|SetStunCooldown (- (Variables|Default|GetStunCooldown) DeltaSeconds))))

(event Input|ActionEvents|InputActionStun
  (params (Key :type Key%20Structure :default "None"))
  (bind _returnvalue (Transformation|GetActorLocation))
  (:Pressed
    (if (<= (Variables|Default|GetStunCooldown) 0.0)
      (Variables|Default|SetStunCooldown (Variables|Default|GetTimeBetweenStuns))
      (Class|MazeCharacter|ActivateStunParticleSystem)
      (bind _outhits (Collision|MultiSphereTraceForObjects _returnvalue _returnvalue (Variables|Default|GetStunTraceRadius) (Variables|Default|GetStunTraceTypes) false 0 "None"))
      (for _array_element _outhits
        (bind _asnpcenemy_bp (Utilities|Casting|CastToNPCEnemyBP (.HitActor (Collision|BreakHitResult _array_element))))
        (Audio|PlaySound2D "/Game/Sound/SFX/SFX_Stun.SFX_Stun" 1.0 1.0 0.0 0 0 false)
        (Default|Stunned _asnpcenemy_bp)))))

(event Input|KeyboardEvents|P
  (params (Key :type Key%20Structure :default "None"))
  (:Pressed
    (Utilities|Casting|CastToMazeGameModeBP (Game|GetGameMode))))

(fn ConstructionScript)

(fn GetStunCooldown
  (return 0.0))