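; AI controller for enemy NPCs that runs the NPCEnemyBT behavior tree and feeds its blackboard.
; On BeginPlay it stores the pawn's starting location as GuardPosition.
; Perception updates write the reported actor to TargetActor, without checking whether it was sensed or lost.
; Each Tick writes the pawn's distance to that target as DistanceToPlayer and prints it on screen for debugging.
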(event OnTargetPerceptionUpdated(AIPerception)
  (params (Actor :type Actor%20Object%20Reference) (Stimulus :type AI%20Stimulus%20Structure))
  (AI|Components|Blackboard|SetValueasObject (AI|GetBlackboard 0) (Utilities|Name|MakeLiteralName "TargetActor") Actor))

(event EventBeginPlay
  (AI|RunBehaviorTree "/Game/NPCEnemyBT.NPCEnemyBT")
  (AI|Components|Blackboard|SetValueasVector (AI|GetBlackboard 0) (Utilities|Name|MakeLiteralName "GuardPosition") (Transformation|GetActorLocation (Pawn|GetControlledPawn))))

(event EventTick
  (params (DeltaSeconds :type Float%20%28single-precision%29))
  (bind _returnvalue (Utilities|Name|MakeLiteralName "TargetActor"))
  (bind _returnvalue_2 (AI|GetBlackboard 0))
  (bind _returnvalue_3 (AI|Components|Blackboard|GetValueasObject _returnvalue_2 _returnvalue))
  (if (Utilities|IsValid _returnvalue_3)
    (bind _asactor (Utilities|Casting|CastToActor _returnvalue_3))
    (AI|Components|Blackboard|SetValueasFloat (AI|GetBlackboard 0) (Utilities|Name|MakeLiteralName "DistanceToPlayer") (Transformation|GetDistanceTo _asactor (Pawn|GetControlledPawn)))
    (Development|PrintString (Utilities|String|ToString(Float) (Transformation|GetDistanceTo _asactor (Pawn|GetControlledPawn))) true false "(R=0.000000,G=0.660000,B=1.000000,A=1.000000)" 0.025)))

(fn ConstructionScript)