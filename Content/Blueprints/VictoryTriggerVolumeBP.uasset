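; Victory trigger volume that records level completion when the maze character overlaps it.
; It finds the current level's index by matching its name against the GameLevels array on MazeGameModeBP.
; If a save game already exists, it writes that index to FurthestCompletedLevel and saves the slot, overwriting the stored value without checking whether it is higher.
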(event EventBeginPlay)

(event Collision|EventActorBeginOverlap
  (params (OtherActor :type Actor%20Object%20Reference))
  (bind _asmaze_character_bp (Utilities|Casting|CastToMazeCharacterBP OtherActor))
  (if (== _asmaze_character_bp OtherActor)
    (bind _returnvalue (Game|GetCurrentLevelName true))
    (bind _asmaze_game_mode_bp (Utilities|Casting|CastToMazeGameModeBP (Game|GetGameMode)))
    (for (_array_element _array_index) (Variables|/Game/MazeGameModeBP.MazeGameModeBP_C|GetGameLevels _asmaze_game_mode_bp)
      (if (Utilities|Enum|Equal(Enum) (Utilities|GetObjectName (Utilities|ResolveSoftReference _array_element)) _returnvalue)
        (bind _returnvalue_2 (SaveGame|DoesSaveGameExist (Variables|Default|GetSlot%20Name)))
        (if _returnvalue_2
          (bind _returnvalue_3 (SaveGame|LoadGamefromSlot (Variables|Default|GetSlot%20Name)))
          (bind _asmaze_save_game_bp (Utilities|Casting|CastToMazeSaveGameBP _returnvalue_3))
          (bind _output_get (Variables|Default|SetAs%20Maze%20Save%20Game%20BP _asmaze_save_game_bp))
          (bind _output_get_2 (Variables|Default|SetArray%20Index _array_index))
          (Variables|/Script/GPE230_PhoenixRoss.MazeSaveGame|SetfurthestCompletedLevel _output_get _output_get_2)
          (SaveGame|SaveGametoSlot _output_get (Variables|Default|GetSlot%20Name)))))))

(event EventTick
  (params (DeltaSeconds :type Float%20%28single-precision%29)))

(fn ConstructionScript)