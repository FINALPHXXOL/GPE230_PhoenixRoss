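; Maze game mode that starts background music and provides functions for level flow and menus.
; LoadNextLevel opens the GameLevels entry following the save's LastCompletedLevel; if none matches, it resets that value and returns to the main menu.
; Separate loaders for levels 1–3 require an existing save and check FurthestCompletedLevel before opening.
; Menu functions create level select, options and pause widgets with a mouse cursor, with pause and resume toggling game pause.
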(event EventBeginPlay
  (Audio|PlaySound2D "/Game/Sound/Music/Music_Katamari.Music_Katamari" 1.0 1.0 0.0 "/Game/Sound/MusicConcurrency.MusicConcurrency" 0 false))

(event EventTick
  (params (DeltaSeconds :type Float%20%28single-precision%29)))

(fn ConstructionScript)

(fn RestartLevel
  (bind _returnvalue (Game|GetCurrentLevelName true))
  (Game|OpenLevel(byName) (Utilities|String|StringToName _returnvalue))
  (return))

(fn LoadNextLevel
  (for _index (range 1 (Utilities|Array|LastIndex (Variables|Default|GetGameLevels)))
    (Variables|Default|SetLevelIndex _index)
    (bind _returnvalue (SaveGame|DoesSaveGameExist (Variables|Default|GetSlot%20Name)))
    (if _returnvalue
      (bind _returnvalue_2 (SaveGame|LoadGamefromSlot (Variables|Default|GetSlot%20Name)))
      (bind _asmaze_save_game_bp (Utilities|Casting|CastToMazeSaveGameBP _returnvalue_2))
      (bind _output_get (Variables|Default|SetAs%20Maze%20Save%20Game%20BP _asmaze_save_game_bp))
      (if (== (Variables|/Script/GPE230_PhoenixRoss.MazeSaveGame|GetlastCompletedLevel _output_get) (- (Variables|Default|GetLevelIndex) 1))
        (Game|OpenLevel(byObjectReference) (Utilities|Array|Get(acopy) (Variables|Default|GetGameLevels) (Variables|Default|GetLevelIndex)))
        (return))))
  (bind _returnvalue_3 (SaveGame|DoesSaveGameExist (Variables|Default|GetSlot%20Name)))
  (if _returnvalue_3
    (bind _returnvalue_4 (SaveGame|LoadGamefromSlot (Variables|Default|GetSlot%20Name)))
    (bind _asmaze_save_game_bp_2 (Utilities|Casting|CastToMazeSaveGameBP _returnvalue_4))
    (bind _output_get_2 (Variables|Default|SetAs%20Maze%20Save%20Game%20BP _asmaze_save_game_bp_2))
    (Variables|/Script/GPE230_PhoenixRoss.MazeSaveGame|SetlastCompletedLevel _output_get_2 0)
    (SaveGame|SaveGametoSlot (Variables|Default|GetAs%20Maze%20Save%20Game%20BP) (Variables|Default|GetSlot%20Name))
    (CallFunction|LoadMainMenu)
    (return)))

(fn LoadMainMenu
  (Game|OpenLevel(byName) "MenuLevel")
  (return))

(fn LoadSelectLevelMenu
  (bind _returnvalue (Game|GetPlayerController 0))
  (bind _returnvalue_2 (UserInterface|CreateWidget "/Game/Blueprints/UI/LevelSelectBP.LevelSelectBP_C" _returnvalue))
  (bind _output_get (Variables|Default|SetSelectLevelUI _returnvalue_2))
  (UserInterface|Viewport|AddtoViewport _output_get 0)
  (Variables|/Script/Engine.PlayerController|SetbShowMouseCursor _returnvalue true)
  (return))

(fn LoadOptionsMenu
  (bind _returnvalue (Game|GetPlayerController 0))
  (bind _returnvalue_2 (UserInterface|CreateWidget "/Game/Blueprints/UI/OptionsBP.OptionsBP_C" _returnvalue))
  (bind _output_get (Variables|Default|SetOptionsUI _returnvalue_2))
  (UserInterface|Viewport|AddtoViewport _output_get 0)
  (Variables|/Script/Engine.PlayerController|SetbShowMouseCursor _returnvalue true)
  (return))

(fn LoadPauseMenu
  (bind _returnvalue (Game|GetPlayerController 0))
  (bind _returnvalue_2 (UserInterface|CreateWidget "/Game/Blueprints/UI/PauseMenuBP.PauseMenuBP_C" _returnvalue))
  (bind _output_get (Variables|Default|SetPauseUI _returnvalue_2))
  (UserInterface|Viewport|AddtoViewport _output_get 0)
  (Variables|/Script/Engine.PlayerController|SetbShowMouseCursor _returnvalue true)
  (Game|SetGamePaused true)
  (return))

(fn ResumeGame
  (Variables|/Script/Engine.PlayerController|SetbShowMouseCursor (Game|GetPlayerController 0) false)
  (Widget|RemovefromParent (Variables|Default|GetPauseUI))
  (Game|SetGamePaused false)
  (return))

(fn LoadLevel1
  (bind _returnvalue (SaveGame|DoesSaveGameExist (Variables|Default|GetSlot%20Name)))
  (if _returnvalue
    (bind _returnvalue_2 (SaveGame|LoadGamefromSlot (Variables|Default|GetSlot%20Name)))
    (bind _asmaze_save_game_bp (Utilities|Casting|CastToMazeSaveGameBP _returnvalue_2))
    (bind _output_get (Variables|Default|SetAs%20Maze%20Save%20Game%20BP _asmaze_save_game_bp))
    (if (>= (Variables|/Script/GPE230_PhoenixRoss.MazeSaveGame|GetfurthestCompletedLevel _output_get) 0)
      (Game|OpenLevel(byObjectReference) (Utilities|Array|Get(acopy) (Variables|Default|GetGameLevels) 1))
      (return)
      (else
        (Development|PrintString "You have not gotten far enough (TODO: add boolean for completed game in MazeSaveGame)")))))

(fn LoadLevel2
  (bind _returnvalue (SaveGame|DoesSaveGameExist (Variables|Default|GetSlot%20Name)))
  (if _returnvalue
    (bind _returnvalue_2 (SaveGame|LoadGamefromSlot (Variables|Default|GetSlot%20Name)))
    (bind _asmaze_save_game_bp (Utilities|Casting|CastToMazeSaveGameBP _returnvalue_2))
    (bind _output_get (Variables|Default|SetAs%20Maze%20Save%20Game%20BP _asmaze_save_game_bp))
    (if (>= (Variables|/Script/GPE230_PhoenixRoss.MazeSaveGame|GetfurthestCompletedLevel _output_get) 1)
      (Game|OpenLevel(byObjectReference) (Utilities|Array|Get(acopy) (Variables|Default|GetGameLevels) 2))
      (return)
      (else
        (Development|PrintString "You have not gotten far enough (TODO: add boolean for completed game in MazeSaveGame)")))))

(fn LoadLevel3
  (bind _returnvalue (SaveGame|DoesSaveGameExist (Variables|Default|GetSlot%20Name)))
  (if _returnvalue
    (bind _returnvalue_2 (SaveGame|LoadGamefromSlot (Variables|Default|GetSlot%20Name)))
    (bind _asmaze_save_game_bp (Utilities|Casting|CastToMazeSaveGameBP _returnvalue_2))
    (bind _output_get (Variables|Default|SetAs%20Maze%20Save%20Game%20BP _asmaze_save_game_bp))
    (if (>= (Variables|/Script/GPE230_PhoenixRoss.MazeSaveGame|GetfurthestCompletedLevel _output_get) 2)
      (Game|OpenLevel(byObjectReference) (Utilities|Array|Get(acopy) (Variables|Default|GetGameLevels) 3))
      (return)
      (else
        (Development|PrintString "You have not gotten far enough (TODO: add boolean for completed game in MazeSaveGame)")))))