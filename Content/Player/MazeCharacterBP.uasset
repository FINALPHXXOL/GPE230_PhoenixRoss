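; MazeCharacterBP is the player character for a maze game, with an area stun ability against enemies.
; The Stun input, when off cooldown, restarts the cooldown, activates a stun particle system and runs a multi-sphere object trace at the character's location.
; Hit actors that cast to NPCEnemyBP receive a Stunned call.
; Tick counts the cooldown down by delta time.
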(event EventBeginPlay)

(event EventTick
  (params (DeltaSeconds :type Float%20%28single-precision%29))
  (if (> (Variables|Default|GetStunCooldown) 0.0)
    (Variables|Default|SetStunCooldown (- (Variables|Default|GetStunCooldown) DeltaSeconds))))

(event Input|ActionEvents|InputActionStun
  (params (Key :type Key%20Structure :default "None"))
  (bind _returnvalue (Transformation|GetActorLocation))
  (:Pressed
    (if (<= (Variables|Default|GetStunCooldown) 0.0)
      (Variables|Default|SetStunCooldown (Variables|Default|GetTimeBetweenStuns))
      (Class|MazeCharacter|ActivateStunParticleSystem)
      (bind _outhits (Collision|MultiSphereTraceForObjects _returnvalue _returnvalue (Variables|Default|GetStunTraceRadius) (Variables|Default|GetStunTraceTypes) false 0 "None"))
      (for _array_element _outhits
        (bind _asnpcenemy_bp (Utilities|Casting|CastToNPCEnemyBP (.HitActor (Collision|BreakHitResult _array_element))))
        (Default|Stunned _asnpcenemy_bp)))))

(fn ConstructionScript)